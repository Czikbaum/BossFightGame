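; Attack component for BP_ThirdPersonCharacter that runs a four-step melee combo: two attacks, a kick and a final attack.
; IA_Attack starts the combo if CanAttack is true, and presses during an attack are buffered in SaveAttack.
; AttackIndex selects each DoOnce-guarded event, which plays its montage after a short delay and advances the index.
; SwordAttackCombo, not called within this graph, either consumes the buffered press to continue or resets through StopCombo.
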(event `self.ReceiveBeginPlay`
  ;[0 0 0] Get Character Mesh
  (bind _asbp_third_person_character (cast `/Game/Blueprints/BP_ThirdPersonCharacter` (`self.GetOwner`)))
  (set `self.CharacterMesh` (`Character.Mesh` _asbp_third_person_character)))

(event `Attack1`
  ;[0 0 0] Attack 1
  (`/Engine/EditorBlueprintResources/StandardMacros.DoOnce` false :!label _label
    (:`Completed`
      (`KismetSystemLibrary.Delay` 0.2)
      (`|PlayMontage` (`self.CharacterMesh`) "/Game/Animations/SwordAttacks/Attack1_Montage.Attack1_Montage" 0.5
        (:`then`
          (set `self.attack Index` 1)
          (goto _label :!via `Reset`))))))

(event `EnhancedInput|/Game/ThirdPerson/Input/Actions/IA_Attack`
  (params (ActionValue :type Boolean) (ElapsedSeconds :type "Float (double-precision)") (TriggeredSeconds :type "Float (double-precision)") (InputAction :type "InputAction Object Reference" :default "/Game/ThirdPerson/Input/Actions/IA_Attack.IA_Attack"))
  ;[0 0 0] Attack Input
  (:`Started`
    (if (`self.can Attack?`)
      (`self.Sword Attack`))))

(event `Attack 2`
  ;[0 0 0] Attack 2
  (`/Engine/EditorBlueprintResources/StandardMacros.DoOnce` false :!label _label_2
    (:`Completed`
      (`KismetSystemLibrary.Delay` 0.2)
      (`|PlayMontage` (`self.CharacterMesh`) "/Game/Animations/SwordAttacks/Attack2_Montage.Attack2_Montage" 0.5
        (:`then`
          (set `self.attack Index` 2)
          (goto _label_2 :!via `Reset`))))))

(event `Sword Attack`
  ;[0 0 0] Sword Attack
  (if (`self.is Attacking?`)
    (set `self.save Attack?` true)
    (else
      (set `self.is Attacking?` true)
      (switch `int` (`self.attack Index`) :!label _label_3
        (:`0`
          (`self.Attack1`))
        (:`1`
          (`self.Attack 2`))
        (:`2`
          (`self.Kick`))
        (:`3`
          (`self.Attack 3`))))))

(event `Kick`
  ;[0 0 0] Kick
  (`/Engine/EditorBlueprintResources/StandardMacros.DoOnce` false :!label _label_4
    (:`Completed`
      (`KismetSystemLibrary.Delay` 0.2)
      (`|PlayMontage` (`self.CharacterMesh`) "/Game/Animations/SwordAttacks/Kick_Montage.Kick_Montage" 0.8
        (:`then`
          (set `self.attack Index` 3)
          (goto _label_4 :!via `Reset`))))))

(event `Sword Attack Combo`
  ;[0 0 0] Combo Continue
  (if (`self.save Attack?`)
    (set `self.save Attack?` false)
    (goto _label_3)
    (else
      (`self.Stop Combo`))))

(event `Attack 3`
  ;[0 0 0] Attack 3
  (`/Engine/EditorBlueprintResources/StandardMacros.DoOnce` false :!label _label_5
    (:`Completed`
      (`KismetSystemLibrary.Delay` 0.2)
      (`|PlayMontage` (`self.CharacterMesh`) "/Game/Animations/SwordAttacks/Attack3_Montage.Attack3_Montage" 0.8
        (:`then`
          (set `self.attack Index` 4)
          (goto _label_5 :!via `Reset`))))))

(event `Stop Combo`
  ;[0 0 0] Combo Stop
  (set `self.is Attacking?` false)
  (set `self.attack Index` 0))