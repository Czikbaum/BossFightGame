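; Player stats component that tracks health and stamina for BP_ThirdPersonCharacter and drives its HUD bars.
; BeginPlay waits a tick, caches the owning character and initializes both bars.
; Functions decrease, restore (capped at max) or raise each stat's maximum, updating the bar directly, with decreases returning true on depletion.
; HealHP sets the HP bar from CurrentSTM / MaxHP rather than from CurrentHP.
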(event `self.ReceiveBeginPlay`
  (`KismetSystemLibrary.DelayUntilNextTick`)
  (bind _asbp_third_person_character (cast `/Game/ThirdPerson/Blueprints/BP_ThirdPersonCharacter` (`self.GetOwner`)))
  (set `self.PlayerCharacterBP` _asbp_third_person_character)
  (`ProgressBar.SetPercent` (`/Game/UI/WB_HUD.STM_Bar` (`/Game/ThirdPerson/Blueprints/BP_ThirdPersonCharacter.HUD_Widget` (`self.PlayerCharacterBP`))) (/ (`self.CurrentSTM`) (`self.MaxSTM`)))
  (`ProgressBar.SetPercent` (`/Game/UI/WB_HUD.HP_Bar` (`/Game/ThirdPerson/Blueprints/BP_ThirdPersonCharacter.HUD_Widget` (`self.PlayerCharacterBP`))) (/ (`self.CurrentHP`) (`self.MaxHP`))))

(fn `Decrease HP`
  (params (DamageTaken :type "Float (double-precision)"))
  (returns (`IsPlayerDead?` :type Boolean))
  (if (not (<= (`self.CurrentHP`) 0.0))
    (set `self.CurrentHP` (- (`self.CurrentHP`) DamageTaken))
    (`ProgressBar.SetPercent` (`/Game/UI/WB_HUD.HP_Bar` (`/Game/ThirdPerson/Blueprints/BP_ThirdPersonCharacter.HUD_Widget` (`self.PlayerCharacterBP`))) (/ (`self.CurrentHP`) (`self.MaxHP`)))
    (if (<= (`self.CurrentHP`) 0.0)
      _
      (else
        (return false))))
  (return true))

(fn `Decrease STM`
  (params (StaminaUsed :type "Float (double-precision)"))
  (returns (NoStaminaLeft :type Boolean))
  (if (not (<= (`self.CurrentSTM`) 0.0))
    (set `self.CurrentSTM` (- (`self.CurrentSTM`) StaminaUsed))
    (`ProgressBar.SetPercent` (`/Game/UI/WB_HUD.STM_Bar` (`/Game/ThirdPerson/Blueprints/BP_ThirdPersonCharacter.HUD_Widget` (`self.PlayerCharacterBP`))) (/ (`self.CurrentSTM`) (`self.MaxSTM`)))
    (if (<= (`self.CurrentSTM`) 0.0)
      _
      (else
        (return false))))
  (return true))

(fn `HealHP`
  (params (HealAmount :type "Float (double-precision)"))
  (set `self.CurrentHP` (+ (`self.CurrentHP`) HealAmount))
  (if (> (`self.CurrentHP`) (`self.MaxHP`))
    (set `self.CurrentHP` (`self.MaxHP`)))
  (`ProgressBar.SetPercent` (`/Game/UI/WB_HUD.HP_Bar` (`/Game/ThirdPerson/Blueprints/BP_ThirdPersonCharacter.HUD_Widget` (`self.PlayerCharacterBP`))) (/ (`self.CurrentSTM`) (`self.MaxHP`))))

(fn `Increase Max STM`
  (params (StaminaIncrease :type "Float (double-precision)"))
  (set `self.MaxSTM` (+ (`self.MaxSTM`) StaminaIncrease))
  (set `self.CurrentSTM` (+ (`self.CurrentSTM`) StaminaIncrease))
  (`ProgressBar.SetPercent` (`/Game/UI/WB_HUD.STM_Bar` (`/Game/ThirdPerson/Blueprints/BP_ThirdPersonCharacter.HUD_Widget` (`self.PlayerCharacterBP`))) (/ (`self.CurrentSTM`) (`self.MaxSTM`))))

(fn `IncreaseMaxHP`
  (params (AdditionalMaxHP :type "Float (double-precision)"))
  (set `self.MaxHP` (+ (`self.MaxHP`) AdditionalMaxHP))
  (bind _output_get (set `self.CurrentHP` (+ (`self.CurrentHP`) AdditionalMaxHP)))
  (`ProgressBar.SetPercent` (`/Game/UI/WB_HUD.HP_Bar` (`/Game/ThirdPerson/Blueprints/BP_ThirdPersonCharacter.HUD_Widget` (`self.PlayerCharacterBP`))) (/ _output_get (`self.MaxHP`))))

(fn `RegenSTM`
  (params (`STM Regen Amount` :type "Float (double-precision)"))
  (set `self.CurrentSTM` (+ (`self.CurrentSTM`) `STM Regen Amount`))
  (if (> (`self.CurrentSTM`) (`self.MaxSTM`))
    (set `self.CurrentSTM` (`self.MaxSTM`)))
  (`ProgressBar.SetPercent` (`/Game/UI/WB_HUD.STM_Bar` (`/Game/ThirdPerson/Blueprints/BP_ThirdPersonCharacter.HUD_Widget` (`self.PlayerCharacterBP`))) (/ (`self.CurrentSTM`) (`self.MaxSTM`))))